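; GM_Player is a game mode Blueprint that runs the end-of-level countdown and restarts the current level.
; A Delay on Tick throttles the logic to roughly once per second.
; Each pass decrements the countdown stored in GI_Game while its end-level flag is set.
; When the countdown equals one, it clears that flag and reopens the current level by name.
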(event EventTick
  (params (DeltaSeconds :type Float%20%28single-precision%29))
  (Utilities|FlowControl|Delay 1.0)
  (bind _asgi_game (Utilities|Casting|CastToGI_Game (Game|GetGameInstance)))
  (if (== (Variables|/Game/GI_Game.GI_Game_C|GetEndLevelCountdown _asgi_game) 1)
    (Variables|/Game/GI_Game.GI_Game_C|SetIsEndLevel _asgi_game false)
    (bind _returnvalue (Game|GetCurrentLevelName true))
    (Game|OpenLevel(byName) (Utilities|String|StringToName _returnvalue)))
  (if (Variables|/Game/GI_Game.GI_Game_C|GetIsEndLevel _asgi_game)
    (Variables|/Game/GI_Game.GI_Game_C|SetEndLevelCountdown _asgi_game (- (Variables|/Game/GI_Game.GI_Game_C|GetEndLevelCountdown _asgi_game) 1))))

(fn ConstructionScript)